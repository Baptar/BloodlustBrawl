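; A test actor that runs the level's intro transition when play begins.
; It shows a connect-loading widget, waits briefly, fades out the music held by the game instance, and plays the loading widget's start animation in reverse.
; When the animation finishes, it removes the loading widget and, after a short delay, adds the start indication UI to the viewport.
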(event EventBeginPlay
  (bind _returnvalue (UserInterface|CreateWidget "/Game/Main/UI/MainMenu/BP_W_ConnectLoading.BP_W_ConnectLoading_C"))
  (UserInterface|Viewport|AddtoViewport _returnvalue 0)
  (Utilities|FlowControl|Delay 1.0)
  (bind _asbp_c_game_instance (Utilities|Casting|CastToBP_C_GameInstance (Game|GetGameInstance)))
  (bind _mysound (Variables|/Script/BloodlustBrawl.C_GameInstance|GetMySound _asbp_c_game_instance)
    (:then
      (Audio|Components|Audio|FadeOut _mysound 2.0 0.0 "Linear" :!class /Script/Engine.AudioComponent))
    (:else
      _))
  (Components|Animation|PlayAnimation _returnvalue (Variables|/Game/Main/UI/MainMenu/BP_W_ConnectLoading.BP_W_ConnectLoading_C|GetStartAnim _returnvalue) 0.0 1 "Reverse"
    (:Finished
      (Widget|RemovefromParent _returnvalue)
      (Utilities|FlowControl|Delay 0.5)
      (bind _returnvalue_2 (UserInterface|CreateWidget "/Game/Main/UI/InGame/UI_IndicationStart.UI_IndicationStart_C"))
      (UserInterface|Viewport|AddtoViewport _returnvalue_2 0))))

(event Collision|EventActorBeginOverlap
  (params (OtherActor :type Actor%20Object%20Reference)))

(event EventTick
  (params (DeltaSeconds :type Float%20%28single-precision%29)))

(fn ConstructionScript)