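; Character Blueprint for Finn the Frog, implementing a special attack that tosses nearby characters into a low-gravity float.
; On input, a sphere trace around Finn finds pawns, launches each character upward and sets its land movement mode to Falling.
; Delays then lower gravity and later restore gravity and walking; sitting inside the loop, they effectively affect only the last character hit.
; The trace leaves persistent debug drawing, and an unconnected launch variant remains.
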(event Input|EnhancedActionEvents|EnhancedInputActionIA_SpecialAttack
  (params (ActionValue :type Boolean) (ElapsedSeconds :type Float%20%28double-precision%29) (TriggeredSeconds :type Float%20%28double-precision%29) (InputAction :type Input%20Action%20Object%20Reference :default "/Game/Main/Blueprint/Input/Actions/IA_SpecialAttack.IA_SpecialAttack"))
  (bind _returnvalue (Transformation|GetActorLocation))
  (:Started
    (bind (_outhits _returnvalue_2) (Collision|MultiSphereTraceForObjects _returnvalue _returnvalue 4e+02 (Utilities|Array|MakeArray "ObjectTypeQuery3") false 0 "Persistent"))
    (if _returnvalue_2
      (for _array_element _outhits
        (bind _ascharacter (Utilities|Casting|CastToCharacter (.HitActor (Collision|BreakHitResult _array_element))))
        (Variables|/Script/Engine.CharacterMovementComponent|SetDefaultLandMovementMode (Variables|/Script/Engine.Character|GetCharacterMovement _ascharacter) "MOVE_Falling")
        (Character|LaunchCharacter _ascharacter "0.000000,0.000000,500.000000" false false)
        (Utilities|FlowControl|Delay 0.1)
        (Variables|/Script/Engine.CharacterMovementComponent|SetGravityScale (Variables|/Script/Engine.Character|GetCharacterMovement _ascharacter) 0.24)
        (Utilities|FlowControl|Delay 2.0)
        (Variables|/Script/Engine.CharacterMovementComponent|SetGravityScale (Variables|/Script/Engine.Character|GetCharacterMovement _ascharacter) 1.75)
        (Variables|/Script/Engine.CharacterMovementComponent|SetDefaultLandMovementMode (Variables|/Script/Engine.Character|GetCharacterMovement _ascharacter) "MOVE_Walking")))))

(fn ConstructionScript)